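; Turret that aims with its owner's camera and fires hitscan shots.
; On BeginPlay it caches the owner as BP_InteractInterace and attaches the muzzle arrow to the fire socket.
; Each tick it rotates the PoseableMesh's root and gun bones to the camera's yaw and pitch.
; Fire line-traces from the muzzle toward the supplied aim ray, spawning impact and muzzle particles only on a hit, without applying damage.
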(event Custom|rotationTurrel
  ;[1 1 1] Comment
  (bind _transform (Default|GetCamera (Variables|Default|GetAs%20BP%20Interact%20Interace)))
  (bind _output_get (Variables|Default|SetTransform _transform))
  (Components|PoseableMesh|SetBoneRotationbyName (Variables|Default|GetPoseableMesh) "root" (Math|Rotator|MakeRotator 0.0 0.0 (.yaw _output_get)) "ComponentSpace")
  (Components|PoseableMesh|SetBoneRotationbyName (Variables|Default|GetPoseableMesh) "gun_jnt" (Math|Rotator|MakeRotator 0.0 (.pitch _output_get) (.yaw _output_get)) "WorldSpace"))

(event EventBeginPlay
  ;[1 1 1] Comment
  (bind _asbp_interact_interace (Utilities|Casting|CastToBP_InteractInterace (Components|GetOwner)))
  (Variables|Default|SetAs%20BP%20Interact%20Interace _asbp_interact_interace)
  (Transformation|AttachComponentToComponent (Variables|Default|GetArrow) (Variables|Default|GetPoseableMesh) "fire" "KeepWorld" "KeepRelative" "KeepRelative" true))

(event EventFire
  (params (Start :type Vector :default "0, 0, 0") (Normal :type Vector :default "0, 0, 0"))
  (bind _arrow (Variables|Default|GetArrow))
  ;[1 1 1] Comment
  (bind (_outhit _returnvalue) (Collision|LineTraceByChannel (Transformation|GetWorldLocation (Variables|Default|GetArrow)) (+ Start (* Normal 5e+05)) "TraceTypeQuery1" false 0 "ForOneFrame"))
  (if _returnvalue
    (Effects|SpawnEmitteratLocation "/Rocket/Mesh/Realistic_Starter_VFX_Pack_Vol2/Particles/Hit/P_Asphalt.P_Asphalt" (.Location (Collision|BreakHitResult _outhit)) (Math|Rotator|MakeRotfromZ (.Normal (Collision|BreakHitResult _outhit))))
    (Effects|SpawnEmitteratLocation "/Rocket/Mesh/Realistic_Starter_VFX_Pack_Vol2/Particles/Hit/P_Concrete.P_Concrete" (Transformation|GetWorldLocation _arrow) (Math|Rotator|MakeRotfromZ (Math|Vector|GetForwardVector _arrow)))))

(event EventTick
  (params (DeltaSeconds :type Float%20%28single-precision%29))
  ;[1 1 1] Comment
  (CallFunction|RotationTurrel))

(fn ConstructionScript)

(fn GetCamera
  (return "0, 0, 0"))